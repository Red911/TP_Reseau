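; Game instance for a network game that owns the player profile and shows the main menu.
; ShowMainMenu creates and caches the menu widget, switches to UI-only input with a cursor, checks for a saved profile and fills in the player name.
; The profile persists through a SaveGame slot, loaded if it exists and otherwise created from current values.
; ChangePlayerName rebuilds the profile, saves it and prints the new name.
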(event `ChangePlayerName`
  (params (PlayerName :type Text))
  (set `self.PlayerProfileInfo` (make `PlayerProfile` PlayerName))
  (`self.SaveProfile`)
  (`KismetSystemLibrary.PrintText` (`.PlayerName` (break `PlayerProfile` (`self.PlayerProfileInfo`))) true true (struct :`G` 0.66 :`B` 1.0 :`A` 1.0) 5.0))

(fn `Check`
  (bind _returnvalue (`GameplayStatics.DoesSaveGameExist` "PlayerProfileSlot"))
  (if _returnvalue
    (`self.Load`)
    (else
      (`self.Save`))))

(fn `Load`
  (bind _returnvalue (`GameplayStatics.LoadGameFromSlot` "PlayerProfileSlot"))
  (bind _assgplayer_profile (cast `SGPlayerProfile` _returnvalue))
  (set `self.PlayerProfileInfo` (`SGPlayerProfile.PlayerProfileStruct` _assgplayer_profile))
  (return))

(fn `Save`
  (`/Engine/EditorBlueprintResources/StandardMacros.IsValid` (`self.PlayerProfile`)
    (:`Is Valid`
      _)
    (:`Is Not Valid`
      (bind _returnvalue (`GameplayStatics.CreateSaveGameObject` "/Script/TP_Reseau.SGPlayerProfile"))
      (set `self.PlayerProfile` _returnvalue)))
  (set `SGPlayerProfile.PlayerProfileStruct` (`self.PlayerProfileInfo`) (`self.PlayerProfile`))
  (`GameplayStatics.SaveGameToSlot` (`self.PlayerProfile`) "PlayerProfileSlot")
  (return))

(fn `ShowMainMenu`
  (bind _returnvalue (`GameplayStatics.GetPlayerController` 0))
  (`/Engine/EditorBlueprintResources/StandardMacros.IsValid` (`self.MainMenuWidget`)
    (:`Is Valid`
      _)
    (:`Is Not Valid`
      (bind _returnvalue_2 (`|CreateWidget` "/Game/Widget/WG_MainMenu.WG_MainMenu_C" _returnvalue))
      (set `self.MainMenuWidget` _returnvalue_2)))
  (`UserWidget.AddToViewport` (`self.MainMenuWidget`) 0)
  (`WidgetBlueprintLibrary.SetInputMode_UIOnlyEx` _returnvalue null)
  (set `PlayerController.bShowMouseCursor` true _returnvalue)
  (`self.CheckForSavedProfile`)
  (`EditableText.SetText` (`/Game/Widget/WG_MainMenu.Input_PlayerName` (`self.MainMenuWidget`)) (`.PlayerName` (break `PlayerProfile` (`self.PlayerProfileInfo`))))
  (return))