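; Menu player controller that handles UI-only input, the lobby screen and leaving a session back to MainMenu.
; InitialSetup loads or creates the saved player profile and passes it to ServerUpdateLobby, which has BP_MenuGameMode refresh the lobby.
; CreateLobby shows a reused WG_Lobby widget, and UpdatePlayerName rebuilds its name list from the supplied profiles.
; EndClientSession destroys the session before opening MainMenu.
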(event `self.ReceiveBeginPlay`
  (if (`self.IsLocalController`)
    (set `self.bShowMouseCursor` true)
    (`WidgetBlueprintLibrary.SetInputMode_UIOnlyEx` self null)))

(event `EndClientSession`
  (`DestroySessionCallbackProxy.DestroySession` self
    (:`then`
      (`GameplayStatics.OpenLevel` "MainMenu"))))

(event `CreateLobby`
  (`self.ShowLobbyMenu`))

(event `InitialSetup`
  (`self.LoadSavedProfile`)
  (`self.ServerUpdateLobby` (`self.PlayerProfile`)))

(event `ServerUpdateLobby`
  (params (PlayerProfile :type "SGPlayerProfile Object Reference"))
  (set `self.PlayerProfile` PlayerProfile)
  (bind _asbp_menu_game_mode (cast `/Game/Framework/Menu/BP_MenuGameMode` (`GameplayStatics.GetGameMode`)))
  (`/Game/Framework/Menu/BP_MenuGameMode.UpdateLobby` _asbp_menu_game_mode true))

(event `UpdatePlayerName`
  (params (PlayerProfiles :type "Array of SGPlayerProfile Object Reference"))
  (`/Engine/EditorBlueprintResources/StandardMacros.IsValid` (`self.Lobby`)
    (:`Is Valid`
      (`/Game/Widget/WG_Lobby.ClearPlayerNames` (`self.Lobby`))
      (`/Game/Widget/WG_Lobby.Update Player Names` (`self.Lobby`) PlayerProfiles))))

(fn `LoadSavedProfile`
  (locals (SlotName :type String :default "PlayerProfile_Slot"))
  (bind _returnvalue (`GameplayStatics.DoesSaveGameExist` (`local.SlotName`)))
  (if (not _returnvalue)
    (bind _returnvalue_2 (`GameplayStatics.CreateSaveGameObject` "/Script/TP_Reseau.SGPlayerProfile"))
    (`GameplayStatics.SaveGameToSlot` _returnvalue_2 (`local.SlotName`)))
  (bind _returnvalue_3 (`GameplayStatics.LoadGameFromSlot` (`local.SlotName`)))
  (bind _assgplayer_profile (cast `SGPlayerProfile` _returnvalue_3))
  (set `self.PlayerProfile` _assgplayer_profile)
  (return))

(fn `ShowLobbyMenu`
  (`/Engine/EditorBlueprintResources/StandardMacros.IsValid` (`self.Lobby`)
    (:`Is Valid`
      _)
    (:`Is Not Valid`
      (bind _returnvalue (`|CreateWidget` "/Game/Widget/WG_Lobby.WG_Lobby_C" (`GameplayStatics.GetPlayerController` 0)))
      (bind _output_get (set `self.Lobby` _returnvalue))))
  (`UserWidget.AddToViewport` _output_get 5)
  (`KismetSystemLibrary.PrintString` (`KismetStringLibrary.Conv_BoolToString` (`Widget.IsVisible` (`self.Lobby`))) true true (struct :`R` 1.0 :`B` 0.096547 :`A` 1.0)))

(fn `UserConstructionScript`)