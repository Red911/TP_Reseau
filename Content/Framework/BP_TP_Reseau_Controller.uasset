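; Network lobby controller that adds the WG_TP2 widget on BeginPlay and runs the pre-match countdown.
; On authority, Tick starts a one-second timer once the Lobby has two players, then travels to Level1 at zero.
; CountDownTime's OnRep updates LobbyMenu, though the created widget is never assigned to it.
; A second counter, apparently left over, resyncs through TimeChecker every ten counts and updates the character's menu.
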(event `self.ReceiveBeginPlay`
  (`self.AddLobbyToServer`))

(event `AddLobbyToServer`
  (`self.AddLobbyToClient`))

(event `AddLobbyToClient`
  (bind _returnvalue (`|CreateWidget` "/Game/Widget/WG_TP2.WG_TP2_C"))
  (`UserWidget.AddToViewport` _returnvalue 0))

(event `self.ReceiveTick`
  (params (DeltaSeconds :type "Float (single-precision)"))
  (`/Engine/EditorBlueprintResources/ActorMacros.Switch Has Authority`
    (:`Authority`
      (bind _returnvalue (`GameplayStatics.GetCurrentLevelName` true))
      (switch `string` _returnvalue
        (:`Lobby`
          (if (`KismetSystemLibrary.IsServer`)
            (bind _returnvalue_2 (`GameModeBase.GetNumPlayers` (`GameplayStatics.GetGameMode`)))
            (if (and (>= _returnvalue_2 2) (not (`self.bHasCountdownStarted `)))
              (`self.StartCountdown`))))
        (:`Level1`
          (`KismetSystemLibrary.K2_PauseTimerHandle` (`self.Timer`)))))))

(event `StartCountdown`
  (set `self.bHasCountdownStarted ` true)
  (bind _returnvalue (`KismetSystemLibrary.K2_SetTimerDelegate` (delegate `TickCountdown`) 1.0 true))
  (set `self.Timer` _returnvalue))

(event `TickCountdown`
  (bind _result (`/Engine/EditorBlueprintResources/StandardMacros.DecrementInt` (`self.Count Down Time`))
    (:`  `
      (if (<= _result 0)
        (`KismetSystemLibrary.K2_ClearAndInvalidateTimerHandle` (`self.Timer`))
        (`NetworkGameInstanceSubSystem.TravelToMap` (subsystem `NetworkGameInstanceSubSystem`) 0 "Level1")
        (else
          (bind _lobbymenu (`self.LobbyMenu`)
            (:`then`
              (`/Game/Widget/WG_Lobby.UpdateTime` _lobbymenu (`self.Count Down Time`)))
            (:`else`)))))))

(fn `DecreaseCounter`
  (bind _result (`/Engine/EditorBlueprintResources/StandardMacros.DecrementInt` (`self.TimeCounter`))
    (:`  `
      (`/Engine/EditorBlueprintResources/ActorMacros.Switch Has Authority`
        (:`Authority`
          (if (== (mod _result 10) 9)
            (set `self.TimeChecker` (`self.TimeCounter`))
            (`self.SetCounter`)
            (else
              (`self.SetCounter`))))
        (:`Remote`
          (`self.SetCounter`))))))

(fn `OnRep_Count Down Time`
  (bind _lobbymenu (`self.LobbyMenu`)
    (:`then`
      (`/Game/Widget/WG_Lobby.UpdateTime` _lobbymenu (`self.Count Down Time`)))
    (:`else`)))

(fn `OnRep_TimeChecker`
  (if (!= (`self.TimeChecker`) (`self.TimeCounter`))
    (set `self.TimeCounter` (`self.TimeChecker`))
    (`KismetSystemLibrary.K2_ClearAndInvalidateTimerHandle` (`self.TimerHandle`))
    (bind _returnvalue (`KismetSystemLibrary.K2_SetTimer` null "DecreaseCounter" 1.0 true))
    (set `self.TimerHandle` _returnvalue)
    (`self.SetCounter`)))

(fn `SetCounter`
  (bind _returnvalue (`self.K2_GetPawn` (`GameplayStatics.GetPlayerController` 0)))
  (bind _lobbymenu (`/Game/ThirdPerson/Blueprints/BP_ThirdPersonCharacter.LobbyMenu` (`self.RefCharacter`)))
  (`/Engine/EditorBlueprintResources/StandardMacros.IsValid` (`self.RefCharacter`)
    (:`Is Valid`
      _)
    (:`Is Not Valid`
      (`/Engine/EditorBlueprintResources/StandardMacros.IsValid` _returnvalue
        (:`Is Valid`
          (bind _asbp_third_person_character (cast `/Game/ThirdPerson/Blueprints/BP_ThirdPersonCharacter` _returnvalue))
          (set `self.RefCharacter` _asbp_third_person_character)))))
  (`/Engine/EditorBlueprintResources/StandardMacros.IsValid` _lobbymenu
    (:`Is Valid`
      (`/Game/Widget/WG_Lobby.UpdateTime` _lobbymenu (`self.TimeCounter`)))))

(fn `UserConstructionScript`)